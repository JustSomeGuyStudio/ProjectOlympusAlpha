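; Networked firearm actor for SKG Shooter Framework, handling firing, fire modes, reloading, ammo, pickup and drop.
; The owning client fires immediately and informs the server, which replicates muzzle transform and firing state so others replay shots.
; Shots use the SKG projectile subsystem, which also feeds optic zeroing, with impacts triggering surface effects and damage messages.
; Full Auto and Burst share one refire timer, and montages drive reload completion.
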(event `Server_SetFireMode`
  (params (FireMode :type "GameplayTag Structure"))
  (if (`BlueprintGameplayTagLibrary.HasTag` (`self.FireModes`) FireMode)
    (set `self.CurrentFireMode` FireMode)))

(event `FireAuto`
  (`self.Fire`))

(event `Server_Fire`
  (params (MuzzleTransform :type "SKGMuzzleTransform Structure"))
  (set `self.FiringReplication` (make `/Game/SKGShooterFramework/Blueprints/DataTypes/ProjectileRepTransform` MuzzleTransform true))
  (`self.Fire`))

(event `/Game/SKGShooterFramework/Blueprints/Interfaces/BPI_Firearm.StopFire`
  (`KismetSystemLibrary.K2_ClearAndInvalidateTimerHandle` (`self.TFire`))
  (`/Engine/EditorBlueprintResources/ActorMacros.Switch Has Authority`
    (:`Authority`
      (set `self.FiringReplication` (make `/Game/SKGShooterFramework/Blueprints/DataTypes/ProjectileRepTransform` (struct :`Location` (0.0 0.0 0.0) :`Direction` (0.0 0.0 0.0)))))
    (:`Remote`
      (`self.Server_StopFire`))))

(event `Server_StopFire`
  (set `self.FiringReplication` (make `/Game/SKGShooterFramework/Blueprints/DataTypes/ProjectileRepTransform` (struct :`Location` (0.0 0.0 0.0) :`Direction` (0.0 0.0 0.0))))
  (`self.StopFire`))

(event `/Game/SKGShooterFramework/Blueprints/Interfaces/BPI_Firearm.CycleFireMode`
  (`self.CycleFireModeImplementation`))

(event `self.SKGFirearm.OnHeld`
  (`self.Set Optic Zeros At Distance`))

(event `self.SKGFirearm.OnProceduralAnimComponentsUpdated`
  (`self.Set Optic Zeros At Distance`))

(event `OnProjectileImpact`
  (params (HitResult :type "HitResult Structure (by ref)") (ImpactDirection :type "Vector Structure") (ProjectileID :type Integer))
  (bind (_bblockinghit _binitialoverlap _time _distance _location _impactpoint _normal _impactnormal _physmat _hitactor) (`GameplayStatics.BreakHitResult` HitResult))
  (bind _asskgphysical_material (cast `SKGPhysicalMaterial` _physmat)
    (:`then`
      (`SKGPhysicalMaterial.PlayEffect` _asskgphysical_material HitResult true (`BlueprintGameplayTagLibrary.MakeLiteralGameplayTag` (struct :`TagName` "Impact.Bullet"))))
    (:`CastFailed`
      _))
  (if (`KismetSystemLibrary.DoesImplementInterface` _hitactor "/Game/SKGShooterFramework/Blueprints/Interfaces/BPI_Hit.BPI_Hit_C")
    (message `/Game/SKGShooterFramework/Blueprints/Interfaces/BPI_Hit.Hit` _hitactor (`self.BaseDamageAmount`) HitResult)))

(event `/Game/SKGShooterFramework/Blueprints/Interfaces/BPI_Interact.Interact`
  (params (Pawn :type "Pawn Object Reference"))
  (`/Engine/EditorBlueprintResources/ActorMacros.Switch Has Authority`
    (:`Authority`
      (if (`self.bCanPickup`)
        (bind _asbp_skgsfexample_pawn (cast `/Game/SKGShooterFramework/Blueprints/Pawn/BP_SKGSFExamplePawn` Pawn))
        (bind _pickedup (`/Game/SKGShooterFramework/Blueprints/Pawn/BP_SKGSFExamplePawn.Pickup Firearm` _asbp_skgsfexample_pawn self))
        (if _pickedup
          (`self.DisablePickup`))))))

(event `/Game/SKGShooterFramework/Blueprints/Interfaces/BPI_Interact.Drop`
  (params (DropPoint :type "/Game/SKGShooterFramework/Blueprints/DataTypes/NetTransform Structure"))
  (`/Engine/EditorBlueprintResources/ActorMacros.Switch Has Authority`
    (:`Authority`
      (set `self.DropLocation` DropPoint)
      (`self.EnablePickup`))))

(event `/Game/SKGShooterFramework/Blueprints/Interfaces/BPI_Interact.EnablePickup`
  (set `self.bCanPickup` true))

(event `/Game/SKGShooterFramework/Blueprints/Interfaces/BPI_Interact.DisablePickup`
  (set `self.bCanPickup` false))

(event `/Game/SKGShooterFramework/Blueprints/Interfaces/BPI_Firearm.Reload`
  (if (> (`self.TotalAmmo`) 0)
    (if (<= (`self.CurrentMagazineAmmo`) 0)
      (`self.PerformReloadMontage` false)
      (else
        (`self.PerformReloadMontage` true)))
    (set `self.bIsReloading` true)
    (`/Engine/EditorBlueprintResources/ActorMacros.Switch Has Authority`
      (:`Remote`
        (`self.Server_Reload`)))))

(event `Server_Reload`
  (set `self.bIsReloading` true))

(event `Server_ReloadComplete`
  (set `self.bIsReloading` false)
  (`self.TransferAmmoToMagazine`))

(event `/Game/SKGShooterFramework/Blueprints/Interfaces/BPI_Firearm.ReloadComplete`
  (if (`self.IsLocallyOwned`)
    (set `self.bIsReloading` false)
    (`self.TransferAmmoToMagazine`)
    (`/Engine/EditorBlueprintResources/ActorMacros.Switch Has Authority`
      (:`Remote`
        (`self.Server_ReloadComplete`)))))

(event `PerformFireMontage`
  (bind _fireanimdata (`self.FireAnimData`))
  (`|PlayMontage` (`self.SkeletalMesh`) (break `/Game/SKGShooterFramework/Blueprints/DataTypes/AnimationMontageData` (break `/Game/SKGShooterFramework/Blueprints/DataTypes/AnimationMontageDataPair` _fireanimdata)) 1.0 0.0 (`.Section_4_88D3D2E14DDEF057FF62B69FD89CC800` (break `/Game/SKGShooterFramework/Blueprints/DataTypes/AnimationMontageData` (break `/Game/SKGShooterFramework/Blueprints/DataTypes/AnimationMontageDataPair` _fireanimdata)))))

(event `PerformReloadMontage`
  (params (bEmptyReload :type Boolean))
  (bind _skeletalmesh (`self.SkeletalMesh`))
  (bind (_reloadanimdata_firearm _reloadanimdata_character) (break `/Game/SKGShooterFramework/Blueprints/DataTypes/AnimationMontageDataPair` (`self.ReloadAnimData`)))
  (bind _reloadanimdata (`self.ReloadAnimData`))
  (bind _reloademptymagazineanimdata (`self.ReloadEmptyMagazineAnimData`))
  (bind (_reloademptymagazineanimdata_firearm _reloademptymagazineanimdata_character) (break `/Game/SKGShooterFramework/Blueprints/DataTypes/AnimationMontageDataPair` (`self.ReloadEmptyMagazineAnimData`)))
  (if bEmptyReload
    (`self.OnReload` _reloadanimdata_character)
    (`|PlayMontage` _skeletalmesh (break `/Game/SKGShooterFramework/Blueprints/DataTypes/AnimationMontageData` (break `/Game/SKGShooterFramework/Blueprints/DataTypes/AnimationMontageDataPair` _reloadanimdata)) 1.0 0.0 (`.Section_4_88D3D2E14DDEF057FF62B69FD89CC800` (break `/Game/SKGShooterFramework/Blueprints/DataTypes/AnimationMontageData` (break `/Game/SKGShooterFramework/Blueprints/DataTypes/AnimationMontageDataPair` _reloadanimdata)))
      (:`OnCompleted`
        _))
    (else
      (`self.OnReload` _reloademptymagazineanimdata_character)
      (`|PlayMontage` _skeletalmesh (break `/Game/SKGShooterFramework/Blueprints/DataTypes/AnimationMontageData` (break `/Game/SKGShooterFramework/Blueprints/DataTypes/AnimationMontageDataPair` _reloademptymagazineanimdata)) 1.0 0.0 (`.Section_4_88D3D2E14DDEF057FF62B69FD89CC800` (break `/Game/SKGShooterFramework/Blueprints/DataTypes/AnimationMontageData` (break `/Game/SKGShooterFramework/Blueprints/DataTypes/AnimationMontageDataPair` _reloademptymagazineanimdata)))
        (:`OnCompleted`
          _))))
  (if (`self.bIsReloading`)
    (`/Engine/EditorBlueprintResources/ActorMacros.Switch Has Authority`
      (:`Remote`
        (`self.Server_ReloadComplete`)))
    (else
      (set `self.bIsReloading` false))))

(fn `CanShoot`
  (returns (CanShoot :type Boolean))
  (if (`self.IsLocallyOwned`)
    (return (and (not (`self.bIsReloading`)) (> (- (`GameplayStatics.GetTimeSeconds`) (`self.TimeStampOfLastShot`)) (`self.FireRate`))))
    (else
      (return true))))

(fn `CycleFireModeImplementation`
  (locals (PreviousFireMode :type "GameplayTag Structure"))
  (bind _firemodes_gameplaytags (break `GameplayTagContainer` (`self.FireModes`)))
  (bind _firemodes_gameplaytags_2 (break `GameplayTagContainer` (`self.FireModes`)))
  (set `local.PreviousFireMode` (`self.CurrentFireMode`))
  (bind _result (`/Engine/EditorBlueprintResources/StandardMacros.IncrementInt` (`self.FireModeIndex`))
    (:`  `
      (if (>= _result (`KismetArrayLibrary.Array_Length` _firemodes_gameplaytags_2))
        (set `self.FireModeIndex` 0))
      (bind _output_get (set `self.CurrentFireMode` (`|GetArrayItem` _firemodes_gameplaytags (`self.FireModeIndex`))))
      (if (!= _output_get (`local.PreviousFireMode`))
        (`/Engine/EditorBlueprintResources/ActorMacros.Switch Has Authority`
          (:`Remote`
            (`self.Server_SetFireMode` (`self.CurrentFireMode`))))))))

(fn `Fire`
  (returns (bSuccess :type Boolean))
  (locals (LocallyOwned :type Boolean) (MuzzleTransform :type "SKGMuzzleTransform Structure"))
  (bind (_fireanimdata_firearm _fireanimdata_character) (break `/Game/SKGShooterFramework/Blueprints/DataTypes/AnimationMontageDataPair` (`self.FireAnimData`)))
  (bind _firingreplication_muzzletransform (break `/Game/SKGShooterFramework/Blueprints/DataTypes/ProjectileRepTransform` (`self.FiringReplication`)))
  (bind _muzzletransform (`local.MuzzleTransform`))
  (if (`self.CanShoot`)
    (set `local.LocallyOwned` (`self.IsLocallyOwned`))
    (if (> (`self.CurrentMagazineAmmo`) 0)
      (if (`local.LocallyOwned`)
        (set `local.MuzzleTransform` (`self.GetMuzzleTransform`))
        (`/Engine/EditorBlueprintResources/ActorMacros.Switch Has Authority`
          (:`Authority`
            (set `self.FiringReplication` (make `/Game/SKGShooterFramework/Blueprints/DataTypes/ProjectileRepTransform` _muzzletransform true)))
          (:`Remote`
            (`self.Server_Fire` _muzzletransform)))
        (`self.FireProjectile` (`local.MuzzleTransform`))
        (`self.PlayFireEffects`)
        (else
          (bind _output_get (set `local.MuzzleTransform` _firingreplication_muzzletransform))
          (`self.FireProjectile` _output_get)
          (`self.PlayFireEffects`)))
      (`|SwitchGameplayTag` (`self.CurrentFireMode`)
        (:`FireModes.FullAuto`
          (bind _returnvalue (`KismetSystemLibrary.K2_SetTimerDelegate` (`|CreateDelegate` :!event `FireAuto`) (`self.FireRate`) :!label _label))
          (set `self.TFire` _returnvalue))
        (:`FireModes.Burst`
          (goto _label))
        (:`FireModes.Semi`
          _))
      (`self.OnFired` (`self.ControlRotationMultiplier`) (`self.RecoilLocationMultiplier`) (`self.RecoilRotationMultiplier`) _fireanimdata_character)
      (set `self.TimeStampOfLastShot` (`GameplayStatics.GetTimeSeconds`))
      (`SKGFirearmComponent.ShotPerformed` (`self.SKGFirearm`))
      (return true)
      (else
        (return false)))))

(fn `FireProjectile`
  (params (MuzzleTransform :type "SKGMuzzleTransform Structure"))
  (`/Engine/EditorBlueprintResources/StandardMacros.DecrementInt` (`self.CurrentMagazineAmmo`)
    (:`  `
      (`SKGProjectileWorldSubsystem.FireProjectile` :`self` (subsystem `SKGProjectileWorldSubsystem`) :`DataAsset` (`self.ProjectileData`) :`ActorsToIgnore` (`self.GetActorsToIgnore`) :`LaunchTransform` (`SKGMuzzleHelpers.MuzzleTransformToTransform` MuzzleTransform) :`OnImpact` (`|CreateDelegate` :!event `OnProjectileImpact`)))))

(fn `GetActorsToIgnore`
  (returns (NewParam :type "Array of Actor Object Reference"))
  (locals (NewLocalVar :type "Array of Actor Object Reference"))
  (bind _array (`|MakeArray` self :!type "Actor Object Reference"))
  (`KismetArrayLibrary.Array_Append` _array (`SKGAttachmentManagerComponent.GetAttachments` (`self.SKGAttachmentManager`)))
  (return _array))

(fn `GetMuzzleTransform`
  (returns (ReturnValue :type "SKGMuzzleTransform Structure"))
  (return (`SKGFirearmComponent.GetMuzzleProjectileTransform` (`self.SKGFirearm`) 100.0 1.0)))

(fn `IsLocallyOwned`
  (returns (ReturnValue :type Boolean))
  (bind _aspawn (cast `Pawn` (`self.GetOwner`))
    (:`then`
      (return (`Pawn.IsLocallyControlled` _aspawn)))
    (:`CastFailed`
      (return false))))

(fn `OnRep_bIsReloading`
  (if (`self.bIsReloading`)
    (if (`self.IsLocallyOwned`)
      _
      (elif (<= (`self.CurrentMagazineAmmo`) 0)
        (`self.PerformReloadMontage` false)
        (else
          (`self.PerformReloadMontage` true))))))

(fn `OnRep_DropLocation`
  (bind (_droplocation_location _droplocation_rotation) (break `/Game/SKGShooterFramework/Blueprints/DataTypes/NetTransform` (`self.DropLocation`)))
  (`self.K2_SetActorLocationAndRotation` _droplocation_location _droplocation_rotation))

(fn `OnRep_FiringReplication`
  (bind (_firingreplication_muzzletransform _firingreplication_bisfiring) (break `/Game/SKGShooterFramework/Blueprints/DataTypes/ProjectileRepTransform` (`self.FiringReplication`)))
  (`/Engine/EditorBlueprintResources/ActorMacros.Switch Has Authority`
    (:`Remote`
      (if _firingreplication_bisfiring
        (`self.Fire`)
        (else
          (`KismetSystemLibrary.K2_ClearAndInvalidateTimerHandle` (`self.TFire`)))))))

(fn `OverrideFireRate`
  (params (NewFireRate :type "Float (double-precision)"))
  (set `self.FireRate` (/ 1.0 (/ NewFireRate 60.0))))

(fn `PlayFireEffects`
  (bind _returnvalue_location (break `SKGMuzzleTransform` (`self.GetMuzzleTransform`)))
  (bind _skeletalmesh (`self.SkeletalMesh`))
  (bind (_returnvalue_location_2 _returnvalue_rotation) (`KismetMathLibrary.BreakTransform` (`SKGFirearmComponent.GetMuzzleTransform` (`self.SKGFirearm`))))
  (bind _currentmuzzlecomponent (`SKGFirearmComponent.CurrentMuzzleComponent` (`self.SKGFirearm`)))
  (`self.PerformFireMontage`)
  (`/Engine/EditorBlueprintResources/StandardMacros.IsValid` _currentmuzzlecomponent
    (:`Is Valid`
      (if (`GameplayTagAssetInterface.HasMatchingGameplayTag` _currentmuzzlecomponent (struct :`TagName` "MuzzleComponentType.Suppressor"))
        (`GameplayStatics.PlaySoundAtLocation` "/Game/SKGShooterFramework/Assets/Firearm/Audio/Shooting/SC_FireSuppressed.SC_FireSuppressed" _returnvalue_location (struct) 1.0 1.0 0.0 null null null null)
        (`NiagaraFunctionLibrary.SpawnSystemAttached` (`self.SuppressedMuzzleEffect`) _skeletalmesh "None" _returnvalue_location_2 _returnvalue_rotation "KeepWorldPosition")
        (else
          (`GameplayStatics.PlaySoundAtLocation` "/Game/SKGShooterFramework/Assets/Firearm/Audio/Shooting/SC_Fire.SC_Fire" _returnvalue_location (struct) 1.0 1.0 0.0 null null null null)
          (`NiagaraFunctionLibrary.SpawnSystemAttached` (`self.MuzzleEffect`) _skeletalmesh "None" _returnvalue_location_2 _returnvalue_rotation "KeepWorldPosition"))))))

(fn `Set Optic Zeros At Distance`
  (bind (_outlocation _returnvalue) (`SKGProjectileWorldSubsystem.GetProjectileLocationAtDistance` (subsystem `SKGProjectileWorldSubsystem`) (`self.ProjectileData`) (`self.ZeroDistanceMeters`) (`SKGMuzzleHelpers.MuzzleTransformToTransform` (`self.GetMuzzleTransform`))))
  (if _returnvalue
    (`SKGFirearmComponent.ZeroOpticsForZeroAtLocation` (`self.SKGFirearm`) _outlocation)
    (else
      (`KismetSystemLibrary.K2_SetTimer` null "Set Optic Zeros At Distance" 0.5))))

(fn `TransferAmmoToMagazine`
  (locals (RequestedAmmo :type Integer) (AmmoReceived :type Integer))
  (bind _returnvalue (`KismetMathLibrary.Clamp` (`local.AmmoReceived`) 0 (`self.MagazineCapacity`)))
  (bind _returnvalue_2 (- (`self.TotalAmmo`) (`local.RequestedAmmo`)))
  (if (or (`self.IsLocallyOwned`) (`self.HasAuthority`))
    (set `local.RequestedAmmo` (- (`self.MagazineCapacity`) (`self.CurrentMagazineAmmo`)))
    (if (< _returnvalue_2 0)
      (set `local.AmmoReceived` (`self.TotalAmmo`))
      (set `self.TotalAmmo` 0)
      (else
        (set `local.AmmoReceived` (`local.RequestedAmmo`))
        (set `self.TotalAmmo` _returnvalue_2)))
    (set `local.AmmoReceived` _returnvalue)
    (set `self.CurrentMagazineAmmo` (`KismetMathLibrary.Clamp` (+ (`self.CurrentMagazineAmmo`) _returnvalue) 0 (`self.MagazineCapacity`)))))

(fn `UserConstructionScript`
  (`self.OverrideFireRate` (`self.FireRate`)))