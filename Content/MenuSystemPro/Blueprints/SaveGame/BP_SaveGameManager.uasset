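; Save game manager, owned by the game instance, that creates, saves, loads and finds numbered slots for the menu system.
; New game and load open the saved level through BPI_GameInstanceExtension, which also exchanges play time.
; Slots can be read without opening a level, letting Continue find the latest timestamp.
; Overridable functions isolate BP_CustomSaveGameObject data: level, save count, play time, timestamp and randomly picked placeholder mission text.
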(fn `AnySaveGameExists`
  (params (SlotPrefix :type String :default "savegame_") (Amount :type Integer :default 20) (UserIndex :type Integer))
  (returns (bSaveGameExists :type Boolean))
  ;[1 1 1] Returns true if any savegame exists in Project/Saved/ folder with the matching slot name
  (for _index (range 1 (+ Amount 1))
    (bind _returnvalue (`GameplayStatics.DoesSaveGameExist` (`KismetStringLibrary.Concat_StrStr` SlotPrefix (`KismetStringLibrary.Conv_IntToString` _index)) UserIndex))
    (if _returnvalue
      (return true)))
  (return false))

(fn `CreateNewGame`
  (params (SlotName :type String) (UserIndex :type Integer) (LevelName :type Name))
  (returns (bSuccess :type Boolean))
  ;[1 1 1] Create New Game
  (bind _returnvalue (`GameplayStatics.DoesSaveGameExist` SlotName UserIndex))
  (if _returnvalue
    (`GameplayStatics.DeleteGameInSlot` SlotName UserIndex))
  (`self.SetInitialCustomSaveGameObjectData` LevelName)
  (bind _returnvalue_2 (`GameplayStatics.SaveGameToSlot` (`self.SaveGameObject`) SlotName UserIndex))
  (`self.LoadGame` SlotName UserIndex)
  (return _returnvalue_2))

(fn `GetLatestSaveGame`
  (params (SlotPrefix :type String :default "savegame_") (UserIndex :type Integer) (Amount :type Integer :default 20))
  (returns (Success :type Boolean) (SlotName :type String))
  (locals (LatestSaveTimestamp :type "DateTime Structure") (LatestSaveSlot :type String))
  ;[1 1 1] Loads the most recent savegame. Used by the 'Continue' button in the Singleplayer Menu
  (for _index (range 1 (+ Amount 1))
    (bind _returnvalue (`KismetStringLibrary.Concat_StrStr` SlotPrefix (`KismetStringLibrary.Conv_IntToString` _index)))
    (bind _returnvalue_2 (`GameplayStatics.DoesSaveGameExist` _returnvalue UserIndex))
    (if _returnvalue_2
      (bind _savegameobject (`self.LoadSaveMetaData` _returnvalue))
      (bind _asbp_custom_save_game_object (cast `/Game/MenuSystemPro/Blueprints/SaveGame/BP_CustomSaveGameObject` _savegameobject))
      (bind _lastsavedtimestamp (`/Game/MenuSystemPro/Blueprints/SaveGame/BP_CustomSaveGameObject.LastSavedTimestamp` _asbp_custom_save_game_object))
      (if (> _lastsavedtimestamp (`local.LatestSaveTimestamp`))
        (set `local.LatestSaveTimestamp` _lastsavedtimestamp)
        (set `local.LatestSaveSlot` _returnvalue))))
  (return (not (`KismetStringLibrary.IsEmpty` (`local.LatestSaveSlot`))) (`local.LatestSaveSlot`)))

(fn `GetLevelFromCustomSaveGameObject`
  (returns (LevelName :type Name))
  ;[1 1 1] Override this function to use your own SaveGame object
  (bind _asbp_custom_save_game_object (cast `/Game/MenuSystemPro/Blueprints/SaveGame/BP_CustomSaveGameObject` (`self.SaveGameObject`)))
  (return (`/Game/MenuSystemPro/Blueprints/SaveGame/BP_CustomSaveGameObject.AreaName` _asbp_custom_save_game_object)))

(fn `Initialize`
  ;[1 1 1] Init
  (cast `/Game/MenuSystemPro/Blueprints/GameFramework/BPI_GameInstanceExtension` (`KismetSystemLibrary.GetOuterObject` self))
  (bind _returnvalue (`GameplayStatics.CreateSaveGameObject` "/Game/MenuSystemPro/Blueprints/SaveGame/BP_CustomSaveGameObject.BP_CustomSaveGameObject_C"))
  (`self.SetCustomSaveGameObject` _returnvalue)
  (return))

(fn `LoadGame`
  (params (SlotName :type String) (UserIndex :type Integer))
  (returns (SaveGameObject :type "SaveGame Object Reference"))
  ;[1 1 1] Load from hard drive
  (bind _output_get (set `self.LastLoadedSaveSlotName` SlotName))
  (bind _returnvalue (`GameplayStatics.LoadGameFromSlot` _output_get UserIndex))
  ;[1 1 1] Set Custom Data
  (`self.SetCustomSaveGameObject` _returnvalue)
  ;[1 1 1] Open Level
  (bind _asbpi_game_instance_extension (cast `/Game/MenuSystemPro/Blueprints/GameFramework/BPI_GameInstanceExtension` (`KismetSystemLibrary.GetOuterObject` self)))
  (`/Game/MenuSystemPro/Blueprints/GameFramework/BPI_GameInstanceExtension.OnOpenLevel` _asbpi_game_instance_extension (`self.GetLevelFromCustomSaveGameObject`) true "")
  (return _returnvalue))

(fn `LoadSaveMetaData`
  (params (SlotName :type String) (UserIndex :type Integer))
  (returns (SaveGameObject :type "SaveGame Object Reference"))
  ;[1 1 1] Load without opening the level, this allows to e.g. setup the Save Game Slots in the Menu
  (bind _returnvalue (`GameplayStatics.LoadGameFromSlot` SlotName UserIndex))
  (return _returnvalue))

(fn `SaveGame`
  (params (SlotName :type String) (UserIndex :type Integer))
  (returns (bSuccess :type Boolean))
  ;[1 1 1] Save variables from the game instance on the save game object
  (`self.SetCustomSaveGameObjectData`)
  ;[1 1 1] Save Game to hard drive
  (bind _returnvalue (`GameplayStatics.SaveGameToSlot` (`self.SaveGameObject`) (`local.SlotName`) (`local.UserIndex`)))
  (return _returnvalue))

(fn `SetCustomSaveGameObject`
  (params (SaveGameObject :type "SaveGame Object Reference"))
  ;[1 1 1] Override this function to use your own SaveGame object
  (bind _asbp_custom_save_game_object (cast `/Game/MenuSystemPro/Blueprints/SaveGame/BP_CustomSaveGameObject` SaveGameObject))
  (set `self.SaveGameObject` _asbp_custom_save_game_object)
  (bind _asbpi_game_instance_extension (cast `/Game/MenuSystemPro/Blueprints/GameFramework/BPI_GameInstanceExtension` (`KismetSystemLibrary.GetOuterObject` self)))
  (`/Game/MenuSystemPro/Blueprints/GameFramework/BPI_GameInstanceExtension.OnSetCurrentPlayTime` _asbpi_game_instance_extension (`/Game/MenuSystemPro/Blueprints/SaveGame/BP_CustomSaveGameObject.PlayTimeInSeconds` _asbp_custom_save_game_object))
  (return))

(fn `SetCustomSaveGameObjectData`
  (bind _savegameobject (`self.SaveGameObject`))
  ;[1 1 1] Set Custom Save Game Object Data while saving. Override this function to use your own SaveGame object
  (bind _asbpi_game_instance_extension (cast `/Game/MenuSystemPro/Blueprints/GameFramework/BPI_GameInstanceExtension` (`KismetSystemLibrary.GetOuterObject` self)))
  (bind _currentlevelname (`/Game/MenuSystemPro/Blueprints/GameFramework/BPI_GameInstanceExtension.GetCurrentLevel` _asbpi_game_instance_extension))
  (set `/Game/MenuSystemPro/Blueprints/SaveGame/BP_CustomSaveGameObject.AreaName` _currentlevelname (`self.SaveGameObject`))
  (set `/Game/MenuSystemPro/Blueprints/SaveGame/BP_CustomSaveGameObject.AreaText` (select `int` (`KismetMathLibrary.RandomIntegerInRange` 0 3) :`0` "Find a way out" :`1` "Escape the town" :`2` "Find Basement Key" :`3` "Find the hiden door" :!type "Name") (`self.SaveGameObject`)) ; Set this dynamically with your game logic \n(e.g. run into a trigger changes this or saving at a certain location)
  (set `/Game/MenuSystemPro/Blueprints/SaveGame/BP_CustomSaveGameObject.SavesCount` (+ (`/Game/MenuSystemPro/Blueprints/SaveGame/BP_CustomSaveGameObject.SavesCount` _savegameobject) 1) _savegameobject)
  (bind _playtimeinseconds (`/Game/MenuSystemPro/Blueprints/GameFramework/BPI_GameInstanceExtension.GetCurrentPlayTime` _asbpi_game_instance_extension))
  (bind _output_get (set `/Game/MenuSystemPro/Blueprints/SaveGame/BP_CustomSaveGameObject.PlayTimeInSeconds` _playtimeinseconds (`self.SaveGameObject`)))
  (`/Game/MenuSystemPro/Blueprints/GameFramework/BPI_GameInstanceExtension.OnSetCurrentPlayTime` _asbpi_game_instance_extension _output_get)
  (set `/Game/MenuSystemPro/Blueprints/SaveGame/BP_CustomSaveGameObject.LastSavedTimestamp` (`KismetMathLibrary.Now`) (`self.SaveGameObject`)))

(fn `SetInitialCustomSaveGameObjectData`
  (params (AreaName :type Name))
  (bind _savegameobject (`self.SaveGameObject`))
  ;[1 1 1] Used when creating a new game. Override this function to use your own SaveGame object
  (set `/Game/MenuSystemPro/Blueprints/SaveGame/BP_CustomSaveGameObject.AreaName` AreaName _savegameobject)
  (set `/Game/MenuSystemPro/Blueprints/SaveGame/BP_CustomSaveGameObject.LastSavedTimestamp` (`KismetMathLibrary.Now`) _savegameobject)
  (set `/Game/MenuSystemPro/Blueprints/SaveGame/BP_CustomSaveGameObject.SavesCount` 1 _savegameobject)
  (set `/Game/MenuSystemPro/Blueprints/SaveGame/BP_CustomSaveGameObject.PlayTimeInSeconds` 0.0 _savegameobject)
  (set `/Game/MenuSystemPro/Blueprints/SaveGame/BP_CustomSaveGameObject.AreaText` (select `int` (`KismetMathLibrary.RandomIntegerInRange` 0 3) :`0` "Find a way out" :`1` "Escape the town" :`2` "Find Basement Key" :`3` "Find the hiden door" :!type "Name") _savegameobject) ; Set this dynamically with your game logic \n(e.g. run into a trigger changes this or saving at a certain location)
)