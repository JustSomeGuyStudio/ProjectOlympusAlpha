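; Game mode component from Menu System Pro that creates and removes local players for split-screen or shared-screen multiplayer.
; In-game spawning gathers PlayerStarts, matches their tags to player indices, then creates each player and spawns the default pawn there.
; Main menu spawning creates only controllers beyond player 0, and both removal functions always keep player 0.
; BeginPlay does nothing, with an unconnected example for spawning players without the menu.
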(event `self.ReceiveBeginPlay`
  ;[1 1 1] Spawn logic to support local multiplayer. Use this if you want to spawn local players without going through the menu - Menu System Pro
)

(fn `GetPlayerStarts`
  (bind _outactors (`GameplayStatics.GetAllActorsOfClass` "/Script/Engine.PlayerStart"))
  (set `self.PlayerSpawnpoints` _outactors))

(fn `RemoveLocalPlayers`
  (locals (CurrentPlayerStart :type "PlayerStart Object Reference") (PlayerIndex :type Integer) (LocalPlayerCount :type Integer :default 0))
  (bind _playercontrollers (`self.PlayerControllers`))
  ;[1 1 1] Remove all local players but the Player Controller with Index 0
  (bind _output_get (set `local.LocalPlayerCount` (`GameplayStatics.GetNumLocalPlayerControllers`)))
  (for _index (range 1 _output_get)
    (if (`KismetArrayLibrary.Array_IsValidIndex` _playercontrollers _index)
      (`KismetArrayLibrary.Array_Remove` _playercontrollers _index))
    (`GameplayStatics.RemovePlayer` (`GameplayStatics.GetPlayerControllerFromID` _index) true)))

(fn `RemoveMainMenuPlayerAtIndex`
  (params (LocalPlayerIndex :type Integer))
  (locals (CurrentPlayerStart :type "PlayerStart Object Reference") (PlayerIndex :type Integer) (LocalPlayerCount :type Integer :default 0))
  (bind _playercontrollers (`self.PlayerControllers`))
  ;[1 1 1] Remove local player at given Index. NOTE: Never removes player 0
  (bind _output_get (set `local.LocalPlayerCount` (`GameplayStatics.GetNumLocalPlayerControllers`)))
  (for _index (range 1 _output_get)
    (if (== _index LocalPlayerIndex)
      (if (`KismetArrayLibrary.Array_IsValidIndex` _playercontrollers _index)
        (`KismetArrayLibrary.Array_Remove` _playercontrollers _index))
      (`GameplayStatics.RemovePlayer` (`GameplayStatics.GetPlayerControllerFromID` _index) true))))

(fn `SpawnIngamePlayers`
  (params (LocalPlayerCount :type Integer :default 2))
  ;[1 1 1] Spawn Players Ingame
  (`self.GetPlayerStarts`)
  (`self.SpawnPlayers` LocalPlayerCount))

(fn `SpawnMainMenuPlayers`
  (params (LocalPlayerCount :type Integer))
  (locals (PlayerIndex :type Integer))
  ;[1 1 1] Create a new local player for every player start in the level and assign a new PlayerController & PlayerCharacter to them.
  (`KismetArrayLibrary.Array_AddUnique` (`self.PlayerControllers`) (`GameplayStatics.GetPlayerControllerFromID` 0)) ; First local player always exists
  (for _index (range 1 LocalPlayerCount)
    (bind _output_get (set `local.PlayerIndex` _index))
    (bind _returnvalue (`GameplayStatics.CreatePlayer` _output_get))
    (`KismetArrayLibrary.Array_AddUnique` (`self.PlayerControllers`) _returnvalue)))

(fn `SpawnPlayers`
  (params (LocalPlayerCount :type Integer))
  (locals (CurrentPlayerStart :type "PlayerStart Object Reference") (PlayerIndex :type Integer))
  ;[1 1 1] Create a new local player for every player start in the level and assign a new PlayerController & PlayerCharacter to them.
  (for _index (range LocalPlayerCount)
    (set `local.PlayerIndex` _index)
    (for (_array_element _array_index) (`self.PlayerSpawnpoints`)
      (if (== (`PlayerStart.PlayerStartTag` _array_element) (`KismetStringLibrary.Conv_StringToName` (`KismetStringLibrary.Conv_IntToString` _index)))
        (bind _returnvalue (`GameplayStatics.CreatePlayer` _array_index))
        (`KismetArrayLibrary.Array_AddUnique` (`self.PlayerControllers`) _returnvalue)
        (bind _returnvalue_2 (`|SpawnActorFromClass` (`GameModeBase.DefaultPawnClass` (`GameplayStatics.GetGameMode`)) (`Actor.GetTransform` _array_element) "AlwaysSpawn" "OverrideRootScale" null null))
        (`Controller.Possess` (`Pawn.GetController` _returnvalue_2) _returnvalue_2)
        (break)))))