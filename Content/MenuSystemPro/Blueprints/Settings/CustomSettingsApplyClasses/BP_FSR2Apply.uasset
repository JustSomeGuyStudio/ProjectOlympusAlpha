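; Settings apply class that turns AMD FidelityFX Super Resolution 2 upscaling on or off from a menu setting value.
; Pre-apply either disables FSR2 or prepares for it by forcing TAA with upsampling and switching DLSS off, saving those dependent settings through the SettingsManager.
; Apply then enables FSR2 via console commands, sets its quality mode and saves the matching screen percentage as resolution scale.
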(event `self.OnPreApply`
  (params (SettingsData :type "/Game/MenuSystemPro/Blueprints/Settings/PDA_SettingsData Object Reference") (Value :type "/Game/MenuSystemPro/Blueprints/Settings/FValueTypes Structure") (SettingsManager :type "/Game/MenuSystemPro/Blueprints/Settings/BP_SettingsManager Object Reference"))
  (bind _string (break `/Game/MenuSystemPro/Blueprints/Settings/FValueTypes` Value))
  ;[1 1 1] FSR2 - Enable AMD FidelityFX Super Resolution 2 Plugin
  (`parent.OnPreApply` SettingsData Value SettingsManager)
  (`|ExecutionSequence`
    (:`then_0`
      (set `self.FSR2Enable` (`KismetMathLibrary.SelectString` "1" "0" (`KismetStringLibrary.NotEqual_StrStr` _string "Off"))))
    (:`then_1`
      (set `self.FSR2Quality` _string))
    (:`then_2`
      (if (`KismetStringLibrary.EqualEqual_StrStr` (`self.FSR2Enable`) "1")
        ;[1 1 1] Set Anti Aliasing Method to Temporal Anti Aliasing (TAA)
        (`KismetSystemLibrary.ExecuteConsoleCommand` (`KismetSystemLibrary.GetOuterObject` self) "r.DefaultFeature.Antialiasing 1" null)
        (`/Game/MenuSystemPro/Blueprints/Settings/BP_SettingsManager.SetStringValue` SettingsManager "/Game/MenuSystemPro/Blueprints/Settings/SettingsData/DA_AntiAliasingMethod.DA_AntiAliasingMethod" "2") ; Save TAA as AA Method to Config
        (`KismetSystemLibrary.ExecuteConsoleCommand` (`KismetSystemLibrary.GetOuterObject` self) "r.AntiAliasingMethod 2" null)
        ;[1 1 1] Enable TAA Upsampling  and TAA Upscaler
        (`KismetSystemLibrary.ExecuteConsoleCommand` (`KismetSystemLibrary.GetOuterObject` self) "r.TemporalAA.Upsampling 1" null)
        (`/Game/MenuSystemPro/Blueprints/Settings/BP_SettingsManager.SetStringValue` SettingsManager "/Game/MenuSystemPro/Blueprints/Settings/SettingsData/DA_TemporalUpsampling.DA_TemporalUpsampling" "1")
        (`KismetSystemLibrary.ExecuteConsoleCommand` (`KismetSystemLibrary.GetOuterObject` self) "r.TemporalAA.Upscaler 1" null)
        ;[1 1 1] Disable other Upscalers, like Nvidia DLSS and Unreal's Temporal Super Resolution (Implemented as AntiAliasing Method).
        (`KismetSystemLibrary.ExecuteConsoleCommand` (`KismetSystemLibrary.GetOuterObject` self) "r.NGX.DLSS.Enable 0" null)
        (`/Game/MenuSystemPro/Blueprints/Settings/BP_SettingsManager.SetStringValue` SettingsManager "/Game/MenuSystemPro/Blueprints/Settings/SettingsData/DA_DLSS.DA_DLSS" "Off") ; Save DLSS Off to file
        (else
          ;[1 1 1] Disable FSR2
          (`KismetSystemLibrary.ExecuteConsoleCommand` (`KismetSystemLibrary.GetOuterObject` self) (`KismetStringLibrary.Concat_StrStr` "r.FidelityFX.FSR2.Enabled " (`self.FSR2Enable`)) null))))))

(event `self.OnApply`
  (params (SettingsData :type "/Game/MenuSystemPro/Blueprints/Settings/PDA_SettingsData Object Reference") (Value :type "/Game/MenuSystemPro/Blueprints/Settings/FValueTypes Structure") (SettingsManager :type "/Game/MenuSystemPro/Blueprints/Settings/BP_SettingsManager Object Reference"))
  (bind _string (break `/Game/MenuSystemPro/Blueprints/Settings/FValueTypes` Value))
  ;[1 1 1] FSR2 - Enable AMD FidelityFX Super Resolution 2 Plugin
  (`parent.OnApply` SettingsData Value SettingsManager)
  (`|ExecutionSequence`
    (:`then_0`
      (set `self.FSR2Enable` (`KismetMathLibrary.SelectString` "1" "0" (`KismetStringLibrary.NotEqual_StrStr` _string "Off"))))
    (:`then_1`
      (set `self.FSR2Quality` _string))
    (:`then_2`
      (switch `string` (`self.FSR2Quality`)
        (:`1`
          (set `self.QualityScreenPercentage` 66.666667))
        (:`2`
          (set `self.QualityScreenPercentage` 58.823529))
        (:`3`
          (set `self.QualityScreenPercentage` 50.0))
        (:`4`
          (set `self.QualityScreenPercentage` 33.333333))))
    (:`then_3`
      (if (`KismetStringLibrary.EqualEqual_StrStr` (`self.FSR2Enable`) "1")
        ;[1 1 1] Enable FSR2 and set the Quality Mode
        (`KismetSystemLibrary.ExecuteConsoleCommand` (`KismetSystemLibrary.GetOuterObject` self) (`KismetStringLibrary.Concat_StrStr` "r.FidelityFX.FSR2.Enabled " (`self.FSR2Enable`)) null)
        (`KismetSystemLibrary.ExecuteConsoleCommand` (`KismetSystemLibrary.GetOuterObject` self) (`KismetStringLibrary.Concat_StrStr` "r.FidelityFX.FSR2.QualityMode " (`self.FSR2Quality`)) null)
        (`KismetSystemLibrary.ExecuteConsoleCommand` (`KismetSystemLibrary.GetOuterObject` self) (`KismetStringLibrary.Concat_StrStr` "r.Screenpercentage " (`KismetStringLibrary.Conv_DoubleToString` (`self.QualityScreenPercentage`))) null)
        (`/Game/MenuSystemPro/Blueprints/Settings/BP_SettingsManager.SetFloatValue` SettingsManager "/Game/MenuSystemPro/Blueprints/Settings/SettingsData/DA_ResolutionScale.DA_ResolutionScale" (`self.QualityScreenPercentage`))))))