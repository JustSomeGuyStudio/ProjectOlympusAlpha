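; Settings apply class for a Boolean NVIDIA DLSS option in MenuSystemPro, which requires the DLSS plugin.
; Both OnPreApply and OnApply are empty, leaving their logic disconnected, so the class currently does nothing.
; The unwired pre-apply logic disables DLSS when false, or on supported hardware sets TAA upsampling and reflection denoising, turns off FSR2 and syncs related settings.
; The unwired apply logic enables DLSS through a console command.
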(event `self.OnPreApply`
  (params (SettingsData :type "/Game/MenuSystemPro/Blueprints/Settings/PDA_SettingsData Object Reference") (Value :type "/Game/MenuSystemPro/Blueprints/Settings/FValueTypes Structure") (SettingsManager :type "/Game/MenuSystemPro/Blueprints/Settings/BP_SettingsManager Object Reference"))
  ;[1 1 1] DLSS - Enable Nvidia DLSS Plugin in your project before using this
)

(event `self.OnApply`
  (params (SettingsData :type "/Game/MenuSystemPro/Blueprints/Settings/PDA_SettingsData Object Reference") (Value :type "/Game/MenuSystemPro/Blueprints/Settings/FValueTypes Structure") (SettingsManager :type "/Game/MenuSystemPro/Blueprints/Settings/BP_SettingsManager Object Reference"))
  ;[1 1 1] DLSS - Enable Nvidia DLSS Plugin in your project before using this
)