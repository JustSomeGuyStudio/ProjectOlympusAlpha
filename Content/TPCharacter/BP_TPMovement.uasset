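; Third-person character movement component with predicted, networked sprint and jump, apparently built on the General Movement Component (GMC) plugin.
; BeginPlay adds the Enhanced Input context, and input events set intent flags that MovementUpdate passes to Jump and Sprint.
; BindReplicationData syncs both flags as client-authoritative inputs and max desired speed as server-authoritative, client-validated output.
; WeaponSelectAnims links unarmed, pistol, rifle or shotgun animation layers by weapon index.
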(event `self.ReceiveBeginPlay`
  (bind _asplayer_controller (cast `PlayerController` (`Pawn.GetController` (`self.GetPawnOwner`))))
  (bind _returnvalue (pcsubsystem `EnhancedInputLocalPlayerSubsystem` _asplayer_controller))
  (`/Engine/EditorBlueprintResources/StandardMacros.IsValid` _returnvalue
    (:`Is Valid`
      (`EnhancedInputSubsystemInterface.AddMappingContext` _returnvalue "/Game/TPCharacter/Input/IMC_TPBaseContext.IMC_TPBaseContext" 0 (struct)))))

(event `EnhancedInput|/Game/TPCharacter/Input/IA_TPSprint`
  (params (ActionValue :type Boolean) (ElapsedSeconds :type "Float (double-precision)") (TriggeredSeconds :type "Float (double-precision)") (InputAction :type "InputAction Object Reference" :default "/Game/TPCharacter/Input/IA_TPSprint.IA_TPSprint"))
  (:`Triggered`
    (set `self.WantsToSprint` true))
  (:`Completed`
    (set `self.WantsToSprint` false)))

(event `EnhancedInput|/Game/TPCharacter/Input/IA_TPJump`
  (params (ActionValue :type Boolean) (ElapsedSeconds :type "Float (double-precision)") (TriggeredSeconds :type "Float (double-precision)") (InputAction :type "InputAction Object Reference" :default "/Game/TPCharacter/Input/IA_TPJump.IA_TPJump"))
  (:`Triggered`
    (set `self.WantsToJump` true))
  (:`Completed`
    (set `self.WantsToJump` false)))

(event `self.BindReplicationData`
  (`parent.BindReplicationData`)
  (`self.BindBool` (`self.WantsToSprint`) "ClientAuth_Input" "CombineIfUnchanged" "Periodic_Output" "NearestNeighbour")
  (`self.BindBool` (`self.WantsToJump`) "ClientAuth_Input" "CombineIfUnchanged" "Periodic_Output" "NearestNeighbour")
  (`self.BindCompressedSinglePrecisionFloat` (`self.MaxDesiredSpeed`) "ServerAuth_Output_ClientValidated" "AlwaysCombine" "None" "Linear"))

(event `self.MovementUpdate`
  (params (DeltaSeconds :type "Float (single-precision)"))
  (`self.Jump` (`self.WantsToJump`) DeltaSeconds)
  (`self.Sprint` (`self.WantsToSprint`) DeltaSeconds))

(event `self.PreMovementUpdate`
  (params (DeltaSeconds :type "Float (single-precision)"))
  (`parent.PreMovementUpdate` DeltaSeconds))

(event `self.MovementUpdateSimulated`
  (params (DeltaSeconds :type "Float (single-precision)"))
  (`parent.MovementUpdateSimulated` DeltaSeconds))

(fn `WeaponSelectAnims`
  (if (== (`self.Weapon`) 0)
    (`SkeletalMeshComponent.LinkAnimClassLayers` (`self.SkeletalMesh`) "/Game/Characters/Heroes/Mannequin/Animations/Locomotion/Unarmed/ABP_UnarmedAnimLayers.ABP_UnarmedAnimLayers_C")
    (elif (== (`self.Weapon`) 1)
      (`SkeletalMeshComponent.LinkAnimClassLayers` (`self.SkeletalMesh`) "/Game/Characters/Heroes/Mannequin/Animations/Locomotion/Pistol/ABP_PistolAnimLayers.ABP_PistolAnimLayers_C")
      (elif (== (`self.Weapon`) 2)
        (`SkeletalMeshComponent.LinkAnimClassLayers` (`self.SkeletalMesh`) "/Game/Characters/Heroes/Mannequin/Animations/Locomotion/Rifle/ABP_RifleAnimLayers.ABP_RifleAnimLayers_C")
        (elif (== (`self.Weapon`) 3)
          (`SkeletalMeshComponent.LinkAnimClassLayers` (`self.SkeletalMesh`) "/Game/Characters/Heroes/Mannequin/Animations/Locomotion/Shotgun/ABP_ShotgunAnimLayers.ABP_ShotgunAnimLayers_C"))))))