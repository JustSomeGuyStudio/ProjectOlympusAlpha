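; FPS player movement component on the General Movement Component (GMC), handling networked jump, sprint and stance.
; Binds client-authoritative input flags plus server-authoritative, client-validated speed and stance for prediction and replication.
; Links the pawn's GMC Ability System and forwards tick and pre-move hooks to it.
; Sprint requires roughly forward movement; cumulative and proxy moves inherit crouch and crawl flags from the last move-history entry.
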(event `self.ReceiveBeginPlay`
  (bind (_returnvalue_x _returnvalue_y _returnvalue_z) (`KismetMathLibrary.BreakVector` (`self.GetRootCollisionExtent` false)))
  (`parent.ReceiveBeginPlay`)
  (set `self.DefaultRadius` _returnvalue_x)
  (set `self.DefaultHalfHeight` _returnvalue_z)
  (set `self.IsCrawling` (`|EnumEquality` (`self.Stance`) "NewEnumerator2"))
  (set `self.BreakingDeceleration` (`self.GetBrakingDeceleration`)))

(event `self.BindReplicationData`
  (`parent.BindReplicationData`)
  (bind _output_get (set `self.AbilitySystem` (`Actor.GetComponentByClass` (`self.GetPawnOwner`) "/Script/GMCAbilitySystem.GMC_AbilitySystemComponent")))
  (set `GMC_AbilitySystemComponent.GMCMovementComponent` self _output_get)
  (`GMC_AbilitySystemComponent.BindReplicationData` (`self.AbilitySystem`))
  (`self.BindBool` (`self.WantsToSprint`) "ClientAuth_Input" "CombineIfUnchanged" "Periodic_Output" "NearestNeighbour")
  (`self.BindBool` (`self.WantsToJump`) "ClientAuth_Input" "CombineIfUnchanged" "Periodic_Output" "NearestNeighbour")
  (`self.BindCompressedSinglePrecisionFloat` (`self.MaxDesiredSpeed`) "ServerAuth_Output_ClientValidated" "AlwaysCombine" "None" "Linear")
  (bind _returnvalue (`self.BindBool` (`self.WantsToCrouch`) "ClientAuth_Input" "CombineIfUnchanged" "Periodic_Output" "NearestNeighbour"))
  (set `self.BI WantsToCrouch` _returnvalue)
  (bind _returnvalue_2 (`self.BindBool` (`self.WantsToCrawl`) "ClientAuth_Input" "CombineIfUnchanged" "Periodic_Output" "NearestNeighbour"))
  (set `self.BI_WantsToCrawl` _returnvalue_2)
  (`self.BindHalfByte` (`self.Stance`) "ServerAuth_Output_ClientValidated" "AlwaysCombine" "Periodic_Output" "NearestNeighbour"))

(event `self.MovementUpdate`
  (params (DeltaSeconds :type "Float (single-precision)"))
  (`self.Jump` (`self.WantsToJump`) DeltaSeconds)
  (`self.Sprint` (`self.WantsToSprint`) DeltaSeconds))

(event `self.Sprint`
  (params (bRequestedSprint :type Boolean) (DeltaSeconds :type "Float (single-precision)"))
  (if (> (`KismetMathLibrary.Dot_VectorVector` (`KismetMathLibrary.Vector_Normal2D` (`self.GetVelocity`)) (`Actor.GetActorForwardVector` (`self.GetGMCPawnOwner`))) 0.5)
    (`parent.Sprint` bRequestedSprint DeltaSeconds)))

(event `self.PreMovementUpdate`
  (params (DeltaSeconds :type "Float (single-precision)"))
  (`parent.PreMovementUpdate` DeltaSeconds))

(event `self.MovementUpdateSimulated`
  (params (DeltaSeconds :type "Float (single-precision)"))
  (`parent.MovementUpdateSimulated` DeltaSeconds))

(event `GMCPlayMontage`
  (params (MontageToPlay :type "AnimMontage Object Reference") (StartPosition :type "Float (single-precision)") (PlayRate :type "Float (single-precision)") (StartSection :type Name) (bInterruptOther :type Boolean) (bCancelOnBlendIn :type Boolean) (bCancelOnBlendOut :type Boolean))
  ;[0.1458 0.1458 0.1458 0.5] GMC Play Montage
  (`|K2Node_PlayMontage` null MontageToPlay StartPosition PlayRate StartSection bInterruptOther bCancelOnBlendIn bCancelOnBlendOut
    (:`OnCompleted`
      (set `self.Montage` null))))

(event `self.PreLocalMoveExecution`
  (params (LocalMove :type "GMC_Move Structure (by ref)"))
  (`parent.PreLocalMoveExecution` LocalMove)
  (`GMC_AbilitySystemComponent.PreLocalMoveExecution` (`self.AbilitySystem`)))

(event `self.GenAncillaryTick`
  (params (DeltaTime :type "Float (single-precision)") (bLocalMove :type Boolean) (bCombinedClientMove :type Boolean))
  (`parent.GenAncillaryTick` DeltaTime bLocalMove bCombinedClientMove)
  (`GMC_AbilitySystemComponent.GenAncillaryTick` (`self.AbilitySystem`) DeltaTime bCombinedClientMove))

(event `self.GenSimulationTick`
  (params (DeltaTime :type "Float (single-precision)"))
  (`parent.GenSimulationTick` DeltaTime)
  (`GMC_AbilitySystemComponent.GenSimulationTick` (`self.AbilitySystem`) DeltaTime))

(event `self.GenPredictionTick`
  (params (DeltaTime :type "Float (single-precision)"))
  (`parent.GenPredictionTick` DeltaTime)
  (`GMC_AbilitySystemComponent.GenPredictionTick` (`self.AbilitySystem`) DeltaTime))

(fn `InitializeCumulativeMove`
  (params (InputState :type "GMC_PawnState Structure (by ref)") (SimStates :type "EGMC_InterpolationStates Enum" :default "Input"))
  (locals (LastIdx :type Integer))
  (bind _bi_wantstocrawl (`self.BI_WantsToCrawl`))
  (bind _bi_wantstocrawl_2 (`self.BI_WantsToCrawl`))
  (bind _bi_wantstocrouch (`self.BI WantsToCrouch`))
  (bind _bi_wantstocrouch_2 (`self.BI WantsToCrouch`))
  (bind (_returnvalue_metadata _returnvalue_inputstate) (break `GMC_Move` (`self.AccessMoveHistory` (`local.LastIdx`))))
  (bind (_returnvalue_metadata_2 _returnvalue_inputstate_2 _returnvalue_outputstate) (break `GMC_Move` (`self.AccessMoveHistory` (`local.LastIdx`))))
  (set `local.LastIdx` (- (`self.GetCurrentMoveHistoryNum`) 1))
  (if (`|EnumEquality` SimStates "Input")
    (`self.SetBoundBool` (`self.GetBoundBool` _bi_wantstocrouch_2 _returnvalue_inputstate) _bi_wantstocrouch_2 InputState)
    (`self.SetBoundBool` (`self.GetBoundBool` _bi_wantstocrawl _returnvalue_inputstate) _bi_wantstocrawl InputState)
    (else
      (`self.SetBoundBool` (`self.GetBoundBool` _bi_wantstocrouch _returnvalue_outputstate) _bi_wantstocrouch InputState)
      (`self.SetBoundBool` (`self.GetBoundBool` _bi_wantstocrawl_2 _returnvalue_outputstate) _bi_wantstocrawl_2 InputState))))

(fn `InitializeProxyMove`
  (params (Move :type "GMC_Move Structure (by ref)"))
  (bind (_metadata _inputstate) (break `GMC_Move` Move))
  (bind _bi_wantstocrouch (`self.BI_WantsToCrouch`))
  (bind _bi_wantstocrawl (`self.BI_WantsToCrawl`))
  (bind _returnvalue (- (`self.GetCurrentMoveHistoryNum`) 1))
  (bind (_returnvalue_metadata _returnvalue_inputstate) (break `GMC_Move` (`self.AccessMoveHistory` _returnvalue)))
  (if (>= _returnvalue 0)
    (`self.SetBoundBool` (`self.GetBoundBool` _bi_wantstocrouch _returnvalue_inputstate) _bi_wantstocrouch _inputstate)
    (`self.SetBoundBool` (`self.GetBoundBool` _bi_wantstocrawl _returnvalue_inputstate) _bi_wantstocrawl _inputstate)))

(fn `OnCumulativeMoveInitialized`
  (params (InputState :type "GMC_PawnState Structure (by ref)") (SimStates :type "EGMC_InterpolationStates Enum" :default "Input") (DeltaTime :type "Float (single-precision)") (Timestamp :type "Float (double-precision)"))
  (returns (ReturnValue :type Boolean))
  (bind _returnvalue (`parent.OnCumulativeMoveInitialized` InputState SimStates DeltaTime Timestamp))
  (`self.InitializeCumulativeMove` InputState SimStates)
  (return _returnvalue))

(fn `SV_OnProxyMoveInitialized`
  (params (Move :type "GMC_Move Structure (by ref)") (DeltaTime :type "Float (single-precision)") (Timestamp :type "Float (double-precision)"))
  (returns (ReturnValue :type Boolean))
  (bind _returnvalue (`parent.SV_OnProxyMoveInitialized` Move DeltaTime Timestamp))
  (`self.InitializeProxyMove` Move)
  (return _returnvalue))