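; BP_PlayerController is the player controller that sets up the local player's HUD and toggles the pose customization panel.
; On BeginPlay, for the local controller only, it creates W_HUD, adds it to the viewport and hands the widget reference to BP_SKGSFHUD.
; Pressing Tab flip-flops the visibility of the HUD's pose customization widget along with the mouse cursor.
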(event `self.ReceiveBeginPlay`
  (if (`self.IsLocalController`)
    (`|ExecutionSequence`
      (:`then_1`
        ;[1 1 1] Adding HUD
        (bind _returnvalue (`|CreateWidget` "/Game/SKGShooterFramework/UI/W_HUD.W_HUD_C"))
        (set `self.W_HUD` _returnvalue)
        (`UserWidget.AddToViewport` _returnvalue 0)
        (bind _asbp_skgsfhud (cast `/Game/SKGShooterFramework/Blueprints/Pawn/BP_SKGSFHUD` (`self.GetHUD`)))
        (set `/Game/SKGShooterFramework/Blueprints/Pawn/BP_SKGSFHUD.W_HUDRef` _returnvalue _asbp_skgsfhud)))))

(event `Key|Tab`
  (params (Key :type "Key Structure"))
  (bind _w_posecustomization (`/Game/SKGShooterFramework/UI/W_HUD.W_PoseCustomization` (`self.W_HUD`)))
  (:`Pressed`
    (`/Engine/EditorBlueprintResources/StandardMacros.FlipFlop`
      (:`A`
        (`Widget.SetVisibility` _w_posecustomization "Visible")
        (set `self.bShowMouseCursor` true))
      (:`B`
        (`Widget.SetVisibility` _w_posecustomization "Hidden")
        (set `self.bShowMouseCursor` false)))))

(fn `UserConstructionScript`)