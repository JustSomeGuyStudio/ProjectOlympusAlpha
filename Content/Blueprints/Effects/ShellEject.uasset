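; Anim notify for weapon shell ejection effects, working on the Niagara effect it has spawned.
; It fetches shell data from the mesh owner, then calls a static mesh override that receives only the effect's display name as variable name, without that data.
; Disconnected nodes hold a fuller version that spawns the shell-eject Niagara system at the ejector socket and feeds it the owner's shell mesh and sound before activation.
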(fn `Received_Notify`
  (params (MeshComp :type "SkeletalMeshComponent Object Reference") (Animation :type "AnimSequenceBase Object Reference") (EventReference :type "AnimNotifyEventReference Structure (by ref)"))
  (returns (ReturnValue :type Boolean))
  (bind (_shellmesh _shellsound) (message `/Game/Blueprints/Interfaces/BPI_NotifyInterface.ShellEject` (`ActorComponent.GetOwner` MeshComp)))
  (bind _returnvalue (`self.GetSpawnedEffect`))
  (`NiagaraFunctionLibrary.OverrideSystemUserVariableStaticMesh` null (`KismetSystemLibrary.GetDisplayName` _returnvalue)))